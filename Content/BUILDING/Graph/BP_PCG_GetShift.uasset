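; Custom PCG Blueprint node in the building graph folder that translates point sets by the location of a reference point.
; It takes the first point of the first InPoint data as the offset, then runs a point loop over every PointsToShift data set.
; Each point has that location added to its own, keeping rotation and scale, and the results leave on ShiftedPoints.
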(fn ExecutewithContext
  (params (InContext :type PCG%20Context%20Structure%20%28by%20ref%29) (Input :type PCG%20Data%20Collection%20Structure%20%28by%20ref%29))
  (bind _returnvalue (Data|GetTypedInputsbyPinLabel Input "InPoint" "/Script/PCG.PCGPointData"))
  (Variables|Default|SetSourcePoint (SpatialData|GetPoint (Utilities|Array|Get(acopy) _returnvalue) 0))
  (bind _returnvalue_2 (Data|GetTypedInputsbyPinLabel Input "PointsToShift" "/Script/PCG.PCGPointData"))
  (for _array_element _returnvalue_2
    (bind _outdata (PCG|FlowControl|PointLoop InContext _array_element 0))
    (Utilities|Array|Add (LocalVariables|GetOutData) (Utilities|Struct|MakePCGTaggedData _outdata 0 "ShiftedPoints")))
  (return (Utilities|Struct|MakePCGDataCollection (LocalVariables|GetOutData))))

(fn PointLoopBody
  (params (InContext :type PCG%20Context%20Structure%20%28by%20ref%29) (InData :type PCG%20Point%20Data%20Object%20Reference) (InPoint :type PCG%20Point%20Structure%20%28by%20ref%29) (OutMetadata :type PCG%20Metadata%20Object%20Reference) (Iteration :type Integer64))
  (bind _transform (Utilities|Struct|BreakPCGPoint InPoint))
  (bind (_location _rotation _scale) (Math|Transform|BreakTransform _transform))
  (bind _structout (Utilities|Struct|SetmembersinPCGPoint InPoint (Math|Transform|MakeTransform (+ _location (.Location (Math|Transform|BreakTransform (.Transform (Utilities|Struct|BreakPCGPoint (Variables|Default|GetSourcePoint)))))) _rotation _scale)))
  (return _structout true))