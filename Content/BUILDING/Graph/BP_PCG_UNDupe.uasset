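; Custom PCG Blueprint node that filters overlapping points out of point data passed from InputPoints to OutPoints.
; ExecuteWithContext runs a point loop on each point data input, and PointLoopBody compares each point against every other in that data.
; A point is rejected when one with a different seed lies within PointDistanceTrashold, so overlapping points with differing seeds are all rejected rather than leaving one.
; Same-seed points are skipped, and the brute-force search scales quadratically.
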(fn ExecutewithContext
  (params (InContext :type PCG%20Context%20Structure%20%28by%20ref%29) (Input :type PCG%20Data%20Collection%20Structure%20%28by%20ref%29))
  (bind _returnvalue (Data|GetInputsbyPinLabel Input "InputPoints"))
  (for _array_element _returnvalue
    (bind _aspcgpoint_data (Utilities|Casting|CastToPCGPointData (.Data (Utilities|Struct|BreakPCGTaggedData _array_element))))
    (bind _outdata (PCG|FlowControl|PointLoop InContext _aspcgpoint_data 0))
    (Utilities|Array|Add (LocalVariables|GetOutData) (Utilities|Struct|MakePCGTaggedData _outdata 0 "OutPoints")))
  (return (Utilities|Struct|MakePCGDataCollection (LocalVariables|GetOutData))))

(fn PointLoopBody
  (params (InContext :type PCG%20Context%20Structure%20%28by%20ref%29) (InData :type PCG%20Point%20Data%20Object%20Reference) (InPoint :type PCG%20Point%20Structure%20%28by%20ref%29) (OutMetadata :type PCG%20Metadata%20Object%20Reference) (Iteration :type Integer64))
  (bind (_transform _density _boundsmin _boundsmax _color _steepness _seed) (Utilities|Struct|BreakPCGPoint InPoint))
  (bind _array_element (Utilities|Array|ForEachLoopwithBreak (SpatialData|GetPoints InData) :!label _label)
    (:LoopBody
      (if (not (== (.Seed (Utilities|Struct|BreakPCGPoint _array_element)) _seed))
        (if (Utilities|Operators|EqualEqual (.location (.Transform (Utilities|Struct|BreakPCGPoint _array_element))) (.location _transform) (Variables|Default|GetPoint%20Distance%20Trashold))
          (LocalVariables|SetPointIsOK false)
          (goto _label Break))))
    (:Completed
      (return InPoint (LocalVariables|GetPointIsOK)))))