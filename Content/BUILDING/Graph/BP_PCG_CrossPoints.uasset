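; Custom PCG Blueprint element for building graphs that expands each input point into four cross-arranged points.
; A variable loop over InPoints data copies each point half a BlockSize along positive and negative X and Y, ignoring point rotation.
; Each copy gets an offset seed and a direction ID from "1" to "4" in a configurable string attribute, then goes to OutPoints.
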(fn ExecutewithContext
  (params (InContext :type PCG%20Context%20Structure%20%28by%20ref%29) (Input :type PCG%20Data%20Collection%20Structure%20%28by%20ref%29))
  (bind _returnvalue (Data|GetInputsbyPinLabel Input "InPoints"))
  (for _array_element _returnvalue
    (bind _aspcgpoint_data (Utilities|Casting|CastToPCGPointData (.Data (Utilities|Struct|BreakPCGTaggedData _array_element))))
    (bind _returnvalue_2 (Metadata|MutableMetadata _aspcgpoint_data))
    (PCG|Metadata|CreateStringAttribute _returnvalue_2 (Variables|Default|GetAttribute%20Name) "not-set" false true)
    (bind _outdata (Class|PCGBlueprintElement|VariableLoop InContext _aspcgpoint_data 0))
    (Utilities|Array|Add (LocalVariables|GetOutData) (Utilities|Struct|MakePCGTaggedData _outdata 0 "OutPoints")))
  (return (Utilities|Struct|MakePCGDataCollection (LocalVariables|GetOutData))))

(fn VariableLoopBody
  (params (InContext :type PCG%20Context%20Structure%20%28by%20ref%29) (InData :type PCG%20Point%20Data%20Object%20Reference) (InPoint :type PCG%20Point%20Structure%20%28by%20ref%29) (OutMetadata :type PCG%20Metadata%20Object%20Reference) (Iteration :type Integer64))
  (bind _block_size (Variables|Default|GetBlock%20Size))
  (Utilities|FlowControl|Sequence
    (:then_0
      (bind _structout (CallFunction|NewFunction InPoint OutMetadata (Metadata|ConstMetadata InData) (* _block_size "0.500000,0.000000,0.000000") "1" 1)))
    (:then_1
      (bind _structout_2 (CallFunction|NewFunction InPoint OutMetadata (Metadata|ConstMetadata InData) (* _block_size "-0.500000,0.000000,0.000000") "2" 2)))
    (:then_2
      (bind _structout_3 (CallFunction|NewFunction InPoint OutMetadata (Metadata|ConstMetadata InData) (* _block_size "0.000000,0.500000,0.000000") "3" 3)))
    (:then_3
      (bind _structout_4 (CallFunction|NewFunction InPoint OutMetadata (Metadata|ConstMetadata InData) (* _block_size "0.000000,-0.500000,0.000000") "4" 4)))
    (:then_4
      (return (Utilities|Array|MakeArray _structout _structout_2 _structout_3 _structout_4)))))

(fn NewFunction
  (params (In%20point :type PCG%20Point%20Structure) (Out%20Metadata :type PCG%20Metadata%20Object%20Reference) (In%20Metadata :type PCG%20Metadata%20Object%20Reference) (Shift :type Vector) (Metadata%20Value :type String) (Seed :type Integer))
  (bind _outpoint (PCG|CopyPoint In%20point true In%20Metadata Out%20Metadata))
  (bind _structout (Utilities|Struct|SetmembersinPCGPoint _outpoint (Math|Transform|MakeTransform (+ (.Location (Math|Transform|BreakTransform (.Transform (Utilities|Struct|BreakPCGPoint _outpoint)))) Shift) (.Rotation (Math|Transform|BreakTransform (.Transform (Utilities|Struct|BreakPCGPoint _outpoint)))) (.Scale (Math|Transform|BreakTransform (.Transform (Utilities|Struct|BreakPCGPoint _outpoint))))) (+ Seed (.Seed (Utilities|Struct|BreakPCGPoint _outpoint)))))
  (Class|PCGMetadataAccessorHelpers|SetStringAttribute _structout Out%20Metadata (Variables|Default|GetAttribute%20Name) Metadata%20Value)
  (return _structout))