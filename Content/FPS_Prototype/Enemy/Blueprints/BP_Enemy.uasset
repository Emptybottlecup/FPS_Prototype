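; Enemy Blueprint for an FPS prototype that takes hits and is destroyed when its health runs out.
; TakeDamage subtracts a fixed amount from HP, then either destroys the actor or plays a hit reaction montage on the mesh.
; A HitReactionCan flag blocks repeated reactions until ReturnHitReactionState re-enables it; nothing in this Blueprint calls that event.
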(event `self.ReceiveBeginPlay`)

(event `Take Damage`
  (bind _output_get (set `self.HP` (- (`self.HP`) 100.0)))
  (if (<= _output_get 0.0)
    (`self.K2_DestroyActor`)
    (elif (`self.bHitReactionCan`)
      (set `self.bHitReactionCan` false)
      (`|PlayMontage` (`self.Mesh`) "/Game/FPS_Prototype/Enemy/Animation/AnimMontage/AM_hit_reaction_Montage.AM_hit_reaction_Montage"))))

(event `ReturnHitReactionState`
  (set `self.bHitReactionCan` true))

(fn `UserConstructionScript`)