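; BP_LiftingGate is a gate actor that rises and lowers when toggled.
; On BeginPlay it stores its starting Z as CurrentHigh.
; The Control event calls Open/Close, where a FlipFlop alternates between playing and reversing a Timeline.
; The Timeline track drives a Lerp on actor Z between the stored height and a fixed offset above it, keeping current X and Y.
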(event `self.ReceiveBeginPlay`
  (bind (_returnvalue_x _returnvalue_y _returnvalue_z) (`KismetMathLibrary.BreakVector` (`self.K2_GetActorLocation`)))
  (`parent.ReceiveBeginPlay`)
  (set `self.CurrentHigh` _returnvalue_z))

(event `self.Control`
  (`self.Open/Close`))

(event `Open/Close`
  (bind (_returnvalue_x _returnvalue_y) (`KismetMathLibrary.BreakVector` (`self.K2_GetActorLocation`)))
  (bind _currenthigh (`self.CurrentHigh`))
  (`/Engine/EditorBlueprintResources/StandardMacros.FlipFlop`
    (:`A`
      (bind (_direction _newtrack_0) (`Timeline|Timeline` :!label _label)
        (:`Update`
          (`self.K2_SetActorLocation` (`KismetMathLibrary.MakeVector` _returnvalue_x _returnvalue_y (`KismetMathLibrary.Lerp` _currenthigh (+ _currenthigh 300.0) _newtrack_0))))))
    (:`B`
      (goto _label :!via `Reverse`))))

(fn `UserConstructionScript`
  (`parent.UserConstructionScript`))