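; BP_LiftingGate1 is a gate actor that slides 300 units along world Y from its starting position when interacted with.
; The interact event plays a timeline whose track lerps the actor's Y between the value cached at BeginPlay and the offset target.
; Tick watches the cached first-person character's mesh and calls Return, reversing the timeline, whenever its world Z is below -200.
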(event `self.ReceiveBeginPlay`
  (bind (_returnvalue_x _returnvalue_y) (`KismetMathLibrary.BreakVector` (`self.K2_GetActorLocation`)))
  (`parent.ReceiveBeginPlay`)
  (set `self.CurrentHigh` _returnvalue_y)
  (bind _asbp_first_person_character (cast `/Game/FPS_Prototype/FirstPerson/Blueprints/BP_FirstPersonCharacter` (`GameplayStatics.GetPlayerPawn` 0)))
  (set `self.As BP First Person Character` _asbp_first_person_character))

(event `self.ReceiveTick`
  (params (DeltaSeconds :type "Float (single-precision)"))
  (bind (_returnvalue_x _returnvalue_y _returnvalue_z) (`KismetMathLibrary.BreakVector` (`SceneComponent.K2_GetComponentLocation` (`/Game/FPS_Prototype/FirstPerson/Blueprints/BP_FirstPersonCharacter.FirstPersonMesh` (`self.As BP First Person Character`)))))
  (if (< _returnvalue_z -200.0)
    (`self.Return`)))

(event `interact`
  (bind (_returnvalue_x _returnvalue_y _returnvalue_z) (`KismetMathLibrary.BreakVector` (`self.K2_GetActorLocation`)))
  (bind _currenthigh (`self.CurrentHigh`))
  (bind (_direction _newtrack_0) (`Timeline|Timeline` :!label _label)
    (:`Update`
      (`self.K2_SetActorLocation` (`KismetMathLibrary.MakeVector` _returnvalue_x (`KismetMathLibrary.Lerp` _currenthigh (+ _currenthigh 300.0) _newtrack_0) _returnvalue_z)))))

(event `Return`
  (goto _label :!via `Reverse`))

(fn `UserConstructionScript`
  (`parent.UserConstructionScript`))