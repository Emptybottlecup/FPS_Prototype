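; BP_Plaid is a trigger actor, apparently a pressure plate, that operates another actor when the first-person player character steps on or off it.
; Its Box component's begin and end overlap events both filter for BP_FirstPersonCharacter, then call Inreract on the ControlledActor reference if it is valid.
; The same call fires on entry and exit, so any on/off state is left to the controlled actor.
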(event `self.Box.OnComponentBeginOverlap`
  (params (OverlappedComponent :type "PrimitiveComponent Object Reference") (OtherActor :type "Actor Object Reference") (OtherComp :type "PrimitiveComponent Object Reference") (OtherBodyIndex :type Integer) (bFromSweep :type Boolean) (SweepResult :type "HitResult Structure (by ref)"))
  (cast `/Game/FPS_Prototype/FirstPerson/Blueprints/BP_FirstPersonCharacter` OtherActor)
  (`/Engine/EditorBlueprintResources/StandardMacros.IsValid` (`self.ControlledActor`)
    (:`Is Valid`
      (`/Game/FPS_Prototype/Walls/BP_NotRichoshetWalls.Inreract` (`self.ControlledActor`)))))

(event `self.Box.OnComponentEndOverlap`
  (params (OverlappedComponent :type "PrimitiveComponent Object Reference") (OtherActor :type "Actor Object Reference") (OtherComp :type "PrimitiveComponent Object Reference") (OtherBodyIndex :type Integer))
  (cast `/Game/FPS_Prototype/FirstPerson/Blueprints/BP_FirstPersonCharacter` OtherActor)
  (`/Engine/EditorBlueprintResources/StandardMacros.IsValid` (`self.ControlledActor`)
    (:`Is Valid`
      (`/Game/FPS_Prototype/Walls/BP_NotRichoshetWalls.Inreract` (`self.ControlledActor`)))))

(fn `UserConstructionScript`)