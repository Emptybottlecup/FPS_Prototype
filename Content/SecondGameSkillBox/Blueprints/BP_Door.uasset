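; BP_Door is a door actor that swings open and can trigger a room change for the first-person player.
; Interact fires a DoOnce with no reset, playing a timeline that lerps yaw a quarter turn from the rotation stored at BeginPlay, while Reverse runs the timeline back.
; A box overlap calls ChangeRoom on the character when DoorNumber is below a fixed cap and matches the character's LevelNumber.
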(event `self.ReceiveBeginPlay`
  (bind (_returnvalue_roll _returnvalue_pitch _returnvalue_yaw) (`KismetMathLibrary.BreakRotator` (`self.K2_GetActorRotation`)))
  (set `self.CurrentRotation` _returnvalue_yaw))

(event `/Game/SecondGameSkillBox/Blueprints/BPI_Interactable.Interact`
  (bind _currentrotation (`self.CurrentRotation`))
  (`/Engine/EditorBlueprintResources/StandardMacros.DoOnce` false
    (:`Completed`
      (bind (_direction _newtrack_0) (`Timeline|Timeline` :!label _label)
        (:`Update`
          (`self.K2_SetActorRotation` (`KismetMathLibrary.MakeRotator` 0.0 0.0 (`KismetMathLibrary.Lerp` _currentrotation (+ _currentrotation -90.0) _newtrack_0))))))))

(event `Reverse`
  (goto _label :!via `Reverse`))

(event `self.Box.OnComponentBeginOverlap`
  (params (OverlappedComponent :type "PrimitiveComponent Object Reference") (OtherActor :type "Actor Object Reference") (OtherComp :type "PrimitiveComponent Object Reference") (OtherBodyIndex :type Integer) (bFromSweep :type Boolean) (SweepResult :type "HitResult Structure (by ref)"))
  (bind _door_number (`self.Door Number`))
  (bind _asbp_first_person_character (cast `/Game/FPS_Prototype/FirstPerson/Blueprints/BP_FirstPersonCharacter` OtherActor))
  (if (and (< _door_number 99) (== _door_number (`/Game/FPS_Prototype/FirstPerson/Blueprints/BP_FirstPersonCharacter.LevelNumber` _asbp_first_person_character)))
    (`/Game/FPS_Prototype/FirstPerson/Blueprints/BP_FirstPersonCharacter.ChangeRoom` _asbp_first_person_character)))

(fn `UserConstructionScript`
  (`parent.UserConstructionScript`))